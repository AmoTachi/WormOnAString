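; Game instance Blueprint that starts and stops playlist music persisting across level transitions.
; PlayPlaylist and StopPlaylist events both call MusicPlaylist, which creates a persistent 2D sound from the given asset.
; Playing starts that sound and stores it in Music without stopping any previous track.
; Stopping logarithmically fades out the stored Music component, regardless of the playlist passed in.
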(event Custom|StopPlaylist
  (params (Playlist :type Sound%20Base%20Object%20Reference))
  (CallFunction|MusicPlaylist true Playlist))

(event Custom|PlayPlaylist
  (params (Playlist :type Sound%20Base%20Object%20Reference))
  (CallFunction|MusicPlaylist false Playlist))

(fn MusicPlaylist
  (params (stopMusic :type Boolean) (Sound :type Sound%20Base%20Object%20Reference))
  (Variables|Default|SetstopMusic stopMusic)
  (bind _returnvalue (Audio|CreateSound2D Sound 1.0 1.0 0.0 0 true))
  (if (Variables|Default|GetstopMusic)
    (Audio|Components|Audio|FadeOut (Variables|Default|Getmusic) 5.0 0.0 "Logarithmic" :!class /Script/Engine.AudioComponent)
    (else
      (Audio|Components|Audio|Play _returnvalue 0.0)
      (Variables|Default|Setmusic _returnvalue))))